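; Hostile animal character that roams, attacks pawns it sees, and becomes a harvestable meat source when killed.
; Wander loops through random reachable points until PawnSensing triggers Chase, which raises walk speed and moves to the target.
; On arrival, a forward sphere trace deals damage and knockback alongside an attack montage.
; Zero health ragdolls it; further player hits add a data-table meat item to inventory until PostHealth depletes and destroys it.
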(event OnSeePawn(PawnSensing)
  (params (Pawn :type Pawn%20Object%20Reference))
  ;[1 1 1] Chase State
  (CallFunction|Chase Pawn))

(event Custom|Wander
  ;[1 1 1] Wander State
  (AI|AIMoveTo self (.RandomLocation (AI|Navigation|GetRandomReachablePointinRadius (Transformation|GetActorLocation) 3.5e+03 0 0)) 0 1.2e+02 false
    (:OnSuccess
      (Utilities|FlowControl|Delay 2.0)
      (CallFunction|Wander))))

(event Custom|Chase
  (params (TargetActor :type Actor%20Object%20Reference))
  (bind _returnvalue (Transformation|GetActorLocation))
  ;[1 1 1] Chase State
  (AI|AIMoveTo self "0, 0, 0" TargetActor 1.2e+02 false
    (:then
      (Variables|/Script/Engine.CharacterMovementComponent|SetMaxWalkSpeed (Variables|Character|GetCharacterMovement) 5e+02))
    (:OnSuccess
      (if (and (not (Variables|Default|GetIsDead?)) (not (Variables|Default|GetIsAttacking?)))
        (Variables|Default|SetIsAttacking? true)
        (Utilities|FlowControl|Sequence
          (:then_0
            (bind (_outhit _returnvalue_2) (Collision|SphereTraceForObjects _returnvalue (+ _returnvalue (* (Math|Vector|GetForwardVector (Transformation|GetActorRotation)) 2.5e+02)) 5e+01 (Utilities|Array|MakeArray "ObjectTypeQuery3") false 0 "None"))
            (if _returnvalue_2
              (Game|Damage|ApplyDamage (.HitActor (Collision|BreakHitResult _outhit)) (Variables|Default|GetAttack%20Damage) 0 0)
              (bind _ascharacter (Utilities|Casting|CastToCharacter (.HitActor (Collision|BreakHitResult _outhit))))
              (Character|LaunchCharacter _ascharacter (+ (* (Math|Vector|GetForwardVector (Transformation|GetActorRotation)) 5e+02) "0.000000,0.000000,50.000000") false false)))
          (:then_1
            (Animation|Montage|PlayMontage (Variables|Character|GetMesh) (Variables|Default|GetAttack%20Montage)
              (:then
                (Audio|PlaySoundatLocation (Variables|Default|GetAttack%20Sound) (Transformation|GetActorLocation) "0, 0, 0" 1.0 1.0 0.0 0 0 0 0))
              (:OnCompleted
                (Variables|Default|SetIsAttacking? false :!label _label))
              (:OnInterrupted
                (goto _label)))))))))

(event EventBeginPlay
  (CallFunction|Wander))

(event Game|Damage|EventAnyDamage
  (params (Damage :type Float%20%28single-precision%29) (DamageType :type Damage%20Type%20Object%20Reference) (InstigatedBy :type Controller%20Object%20Reference) (DamageCauser :type Actor%20Object%20Reference))
  (bind _meatrow (Variables|Default|GetMeatRow))
  ;[1 1 1] Health And Meat Harvest
  (if (not (Variables|Default|GetIsDead?))
    (Variables|Default|SetHealth (- (Variables|Default|GetHealth) Damage))
    (if (<= (Variables|Default|GetHealth) 0.0)
      (Pawn|Components|CharacterMovement|DisableMovement (Variables|Character|GetCharacterMovement))
      (Physics|SetSimulatePhysics (Variables|Character|GetMesh) true)
      (Variables|Default|SetIsDead? true))
    (else
      (bind _returnvalue (Utilities|GetDataTableRow (.datatable _meatrow) (.rowname _meatrow))
        (:then
          (bind _asplayer_char_bp (Utilities|Casting|CastToPlayerChar_BP DamageCauser))
          (Default|AddItem (Variables|/Game/Player/PlayerChar_BP.PlayerChar_BP_C|GetInventory_BPC _asplayer_char_bp) _returnvalue)
          (Variables|Default|SetPostHealth (- (Variables|Default|GetPostHealth) 1.0))
          (if (<= (Variables|Default|GetPostHealth) 0.0)
            (Actor|DestroyActor)))))))

(fn ConstructionScript)
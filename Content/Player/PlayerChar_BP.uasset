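; Player character Blueprint that sets up the on-screen UI, menus and death handling.
; BeginPlay adds the player and objective widgets to the viewport, while a Death event ragdolls the mesh and disables input.
; Craft input toggles the crafting widget through a FlipFlop, switching cursor and input mode.
; Pause input opens a menu, pauses the game and binds its continue button to restore gameplay.
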(event Custom|OnClicked_Event
  (bind _returnvalue (Game|GetPlayerController 0))
  ;[1 1 1] Pause Menu Button
  ;;[1 1 1] Pause Contine Button
  (Widget|RemovefromParent (stale Input|ActionEvents|InputActionPauseGame _returnvalue_2))
  (Variables|/Script/Engine.PlayerController|SetbShowMouseCursor _returnvalue false)
  (Input|SetInputModeGameOnly _returnvalue false)
  (Class|WidgetBlueprintLibrary|SetFocustoGameViewport)
  (Game|SetGamePaused false))

(event Custom|Death
  ;[1 1 1] Death Animation
  (Physics|SetSimulatePhysics (Variables|Character|GetMesh) true)
  (Input|DisableInput 0))

(event EventBeginPlay
  ;[1 1 1] Implement Player UI at BeginPlay
  (Utilities|FlowControl|Sequence
    (:then_0
      (bind _returnvalue (UserInterface|CreateWidget "/Game/Widgets/Player_W.Player_W_C"))
      (bind _output_get (Variables|Default|SetplayerUI _returnvalue))
      (UserInterface|Viewport|AddtoViewport _output_get 0)
      (bind _returnvalue_2 (UserInterface|CreateWidget "/Game/Widgets/Objective_W.Objective_W_C"))
      (bind _output_get_2 (Variables|Default|SetobjWidget _returnvalue_2))
      (UserInterface|Viewport|AddtoViewport _output_get_2 0))))

(event Collision|EventActorBeginOverlap
  (params (OtherActor :type Actor%20Object%20Reference)))

(event EventTick
  (params (DeltaSeconds :type Float%20%28single-precision%29)))

(event Input|ActionEvents|InputActionCraftMenu
  (params (Key :type Key%20Structure :default "None"))
  (bind _returnvalue (Game|GetPlayerController 0))
  ;[1 1 1] Crafting Menu Toggle
  (:Pressed
    (Utilities|FlowControl|FlipFlop
      (:A
        (bind _returnvalue_2 (UserInterface|CreateWidget "/Game/Widgets/Crafting_W.Crafting_W_C"))
        (UserInterface|Viewport|AddtoViewport _returnvalue_2 0)
        (Variables|/Script/Engine.PlayerController|SetbShowMouseCursor _returnvalue true)
        (Input|SetInputModeGameandUI _returnvalue _returnvalue_2 "DoNotLock" true false))
      (:B
        (Widget|RemovefromParent _returnvalue_2)
        (Variables|/Script/Engine.PlayerController|SetbShowMouseCursor _returnvalue false)
        (Input|SetInputModeGameOnly _returnvalue false)
        (Class|WidgetBlueprintLibrary|SetFocustoGameViewport)))))

(event Input|ActionEvents|InputActionPauseGame
  (params (Key :type Key%20Structure :default "None"))
  (bind _returnvalue (Game|GetPlayerController 0))
  ;[1 1 1] Pause Menu Button
  (:Pressed
    (bind _returnvalue_2 (UserInterface|CreateWidget "/Game/Widgets/PauseMenu_W.PauseMenu_W_C"))
    (Utilities|FlowControl|Sequence
      (:then_0
        (UserInterface|Viewport|AddtoViewport _returnvalue_2 0)
        (Variables|/Script/Engine.PlayerController|SetbShowMouseCursor _returnvalue true)
        (Input|SetInputModeGameandUI _returnvalue _returnvalue_2 "DoNotLock" true false)
        (Game|SetGamePaused true))
      (:then_1
        ;;[1 1 1] Pause Contine Button
        (EventDispatchers|AssignOnClicked (Variables|/Game/Widgets/PauseMenu_W.PauseMenu_W_C|GetcontBtn _returnvalue_2) (delegate Custom|OnClicked_Event))))))

(fn ConstructionScript)
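; Player component that runs the Action input: attacking and harvesting, confirming build placement, or eating, chosen by the equipped item's name.
; Attacks play a montage whose notify fires a camera-forward sphere trace, applying damage and effects, sending chop messages to foliage and reacting to Animal-tagged components.
; Building pieces and food are removed from the inventory component on use, with food also restoring hunger, plus thirst for coconuts.
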(event Custom|AttackAndHarvest
  (bind _returnvalue (Game|GetPlayerCameraManager 0))
  (bind _returnvalue_2 (Transformation|GetActorLocation _returnvalue))
  ;[1 1 1] Attack And Harvest
  (Variables|Default|GetInventory%20Widget
    (:then)
    (:else
      (if (Variables|Default|GetCanAttack?)
        (Animation|Montage|PlayMontage (Variables|/Script/Engine.Character|GetMesh (Variables|Default|GetPlayer%20Char%20BP)) "/Game/Characters/Mannequins/Animations/Manny/MM_Attack_Montage.MM_Attack_Montage"
          (:then
            (Variables|Default|SetCanAttack? false)
            (Audio|PlaySoundatLocation "/Game/Audio/Sounds/Whoosh_MS.Whoosh_MS" (Transformation|GetActorLocation (Components|GetOwner)) "0, 0, 0" 1.0 1.0 0.0 0 0 0 0))
          (:OnCompleted
            (Variables|Default|SetCanAttack? true :!label _label))
          (:OnInterrupted
            (goto _label))
          (:OnNotifyBegin
            (bind (_outhit _returnvalue_3) (Collision|SphereTraceForObjects _returnvalue_2 (+ _returnvalue_2 (* (Math|Vector|GetForwardVector (Transformation|GetActorRotation _returnvalue)) 2.5e+02)) 3e+01 (Utilities|Array|MakeArray "ObjectTypeQuery2" "ObjectTypeQuery1" "ObjectTypeQuery3") false (Utilities|Array|MakeArray (Components|GetOwner)) "None"))
            (if _returnvalue_3
              (Game|Damage|ApplyDamage (.HitActor (Collision|BreakHitResult _outhit)) 1e+01 0 (Components|GetOwner))
              (Niagara|SpawnSystematLocation "/Game/NiagaraEffects/Hit_NS.Hit_NS" (.Location (Collision|BreakHitResult _outhit)) "0, 0, 0" "1.000000,1.000000,1.000000" true true "AutoRelease")
              (Audio|PlaySoundatLocation "/Game/Audio/Sounds/Hit_MS.Hit_MS" (.Location (Collision|BreakHitResult _outhit)) "0, 0, 0" 1.0 1.0 0.0 0 0 0 0)
              (if (Utilities|DoesObjectImplementInterface (.HitComponent (Collision|BreakHitResult _outhit)) "/Game/Blueprints/FoliageInteraction_BPI.FoliageInteraction_BPI_C")
                (Class|FoliageInteractionBPI|Chop(Message) (.HitComponent (Collision|BreakHitResult _outhit)) 1e+01 _outhit)
                (else
                  (Utilities|IsValid (.HitComponent (Collision|BreakHitResult _outhit))
                    (:Is%20Valid
                      (if (Components|ComponentHasTag (.HitComponent (Collision|BreakHitResult _outhit)) "Animal")
                        (Audio|PlaySoundatLocation "/Game/Audio/Sounds/Animal_Grunt_MS.Animal_Grunt_MS" (.Location (Collision|BreakHitResult _outhit)) "0, 0, 0" 1.0 1.0 0.0 0 0 0 0)
                        (Niagara|SpawnSystematLocation 0 (.Location (Collision|BreakHitResult _outhit)) "0, 0, 0" "1.000000,1.000000,1.000000" true true "AutoRelease")))))))))))))

(event Custom|Build
  (bind _inventory_bpc (Variables|Default|GetInventory%20BPC))
  (bind _player_char_bp (Variables|Default|GetPlayer%20Char%20BP))
  ;[1 1 1] Attack And Harvest
  (Utilities|FlowControl|DelayUntilNextTick)
  (bind _nomoreleft_ (Default|RemoveItem _inventory_bpc (Variables|/Game/Blueprints/Inventory/Inventory_BPC.Inventory_BPC_C|GetEquippedItem _inventory_bpc) true))
  (if _nomoreleft_
    (Default|EquipItemMesh _player_char_bp)
    (Default|StopBuildMode (Variables|/Game/Player/PlayerChar_BP.PlayerChar_BP_C|GetBuilding_BPC _player_char_bp))))

(event Custom|Eat
  ;[1 1 1] Eat
  (Class|PlayerChar|SetHunger (Variables|Default|GetPlayer%20Char%20BP) 3e+01)
  (if (Utilities|Enum|Equal(Enum) (.name (Variables|/Game/Blueprints/Inventory/Inventory_BPC.Inventory_BPC_C|GetEquippedItem (Variables|Default|GetInventory%20BPC))) "Coconut")
    (Class|PlayerChar|SetThirst (Variables|Default|GetPlayer%20Char%20BP) 3e+01)
    (CallFunction|Eating "/Game/Audio/Sounds/Drink_MS.Drink_MS")
    (else
      (CallFunction|Eating "/Game/Audio/Sounds/Eat_MS.Eat_MS"))))

(event Custom|Eating
  (params (Sound :type Sound%20Base%20Object%20Reference))
  (bind _inventory_bpc (Variables|Default|GetInventory%20BPC))
  ;[1 1 1] Eating
  (Audio|PlaySoundatLocation Sound (Transformation|GetActorLocation (Components|GetOwner)) "0, 0, 0" 1.0 1.0 0.0 0 0 0 0)
  (Animation|Montage|PlayMontage (Variables|/Script/Engine.Character|GetMesh (Variables|Default|GetPlayer%20Char%20BP)) "/Game/Characters/Mannequins/Animations/Manny/MM_Consume_Montage.MM_Consume_Montage"
    (:then
      (bind _nomoreleft_ (Default|RemoveItem _inventory_bpc (Variables|/Game/Blueprints/Inventory/Inventory_BPC.Inventory_BPC_C|GetEquippedItem _inventory_bpc) true))
      (if _nomoreleft_
        (bind _output_get (Variables|/Game/Blueprints/Inventory/Inventory_BPC.Inventory_BPC_C|SetEquippedItem (Variables|Default|GetInventory%20BPC) ""))
        (Default|EquipItemMesh (Variables|Default|GetPlayer%20Char%20BP) _output_get)))))

(event EventBeginPlay
  ;[1 1 1] Initialize Variables
  (bind _asplayer_char_bp (Utilities|Casting|CastToPlayerChar_BP (Components|GetOwner)))
  (Variables|Default|SetPlayer%20Char%20BP _asplayer_char_bp)
  (Variables|Default|SetInventory%20BPC (Variables|/Game/Player/PlayerChar_BP.PlayerChar_BP_C|GetInventory_BPC (Variables|Default|GetPlayer%20Char%20BP)))
  (Variables|Default|SetInventory%20Widget (Variables|/Game/Blueprints/Inventory/Inventory_BPC.Inventory_BPC_C|GetInventory%20Widget (Variables|Default|GetInventory%20BPC))))

(event Input|ActionEvents|InputActionAction
  (params (Key :type Key%20Structure :default "None"))
  (bind _player_char_bp (Variables|Default|GetPlayer%20Char%20BP))
  (bind _building_bpc (Variables|/Game/Player/PlayerChar_BP.PlayerChar_BP_C|GetBuilding_BPC _player_char_bp))
  ;[1 1 1] Attack And Harvest
  (:Pressed
    (if (Variables|/Game/Building/Building_BPC.Building_BPC_C|GetInBuildMode? _building_bpc)
      (Default|BuildPlacement _building_bpc))
    (switch string (.Name (Utilities|Struct|BreakItem_S (Variables|/Game/Blueprints/Inventory/Inventory_BPC.Inventory_BPC_C|GetEquippedItem (Variables|Default|GetInventory%20BPC))))
      (:Default
        (CallFunction|AttackandHarvest))
      (:Floor
        (CallFunction|Build :!label _label))
      (:Wall
        (goto _label))
      (:Window
        (goto _label))
      (:Doorway
        (goto _label))
      (:Coconut
        (CallFunction|Eat :!label _label_2))
      (:Meat
        (goto _label_2)))))
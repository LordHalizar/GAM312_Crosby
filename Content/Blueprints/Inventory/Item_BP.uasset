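; Item_BP is a pickup item actor whose data and mesh come from the Items_DB data table.
; The construction script looks up the row set in ItemRow or, when RandomItem is on, picks Wood or Stone at random, then stores it as Item and applies its static mesh.
; PickupItem returns the stored Item and always allows pickup, and the event graph holds no active logic.
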(event EventBeginPlay)

(event Collision|EventActorBeginOverlap
  (params (OtherActor :type Actor%20Object%20Reference)))

(event EventTick
  (params (DeltaSeconds :type Float%20%28single-precision%29)))

(fn ConstructionScript
  (if (not (Variables|Default|GetRandomItem?))
    (bind _returnvalue (Utilities|GetDataTableRow "/Game/Blueprints/Inventory/Items_DB.Items_DB" (.rowname (Variables|Default|GetItemRow)))
      (:then
        (Variables|Default|SetItem _returnvalue)))
    (else
      (bind _returnvalue_2 (Utilities|GetDataTableRow "/Game/Blueprints/Inventory/Items_DB.Items_DB" (.OutItem (Utilities|Array|Random (Utilities|Array|MakeArray "Wood" "Stone"))))
        (:then
          (Variables|Default|SetItem _returnvalue_2)))))
  (Components|StaticMesh|SetStaticMesh (Variables|Default|GetStaticMesh) (.StaticMesh (Utilities|Struct|BreakItem_S (Variables|Default|GetItem)))))

(fn PickupItem
  (return (Variables|Default|GetItem) true))
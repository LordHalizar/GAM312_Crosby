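; Resource_BP is a harvestable resource for the inventory system that yields items when damaged.
; On AnyDamage from a causer implementing Inventory_BPI, it reduces Health and destroys itself once Health is depleted, with no yield on that final hit.
; On each non-final hit, it looks up ItemName in the Items_DB data table and sends the causer a random small amount of that item via HarvestItemMessage.
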(event Game|Damage|EventAnyDamage
  (params (Damage :type Float%20%28single-precision%29) (DamageType :type Damage%20Type%20Object%20Reference) (InstigatedBy :type Controller%20Object%20Reference) (DamageCauser :type Actor%20Object%20Reference))
  (if (Utilities|DoesObjectImplementInterface DamageCauser "/Game/Blueprints/Inventory/Inventory_BPI.Inventory_BPI_C")
    (bind _output_get (Variables|Default|SetHealth (- (Variables|Default|GetHealth) Damage)))
    (if (<= _output_get 0.0)
      (Actor|DestroyActor)
      (else
        (bind _returnvalue (Utilities|GetDataTableRow "/Game/Blueprints/Inventory/Items_DB.Items_DB" (Variables|Default|GetItemName))
          (:then
            (Class|InventoryBPI|HarvestItem(Message) DamageCauser (Utilities|Struct|MakeItem_S (.Name (Utilities|Struct|BreakItem_S _returnvalue)) (Math|Random|RandomIntegerinRange 2 5) (.StaticMesh (Utilities|Struct|BreakItem_S _returnvalue)) (.Icon (Utilities|Struct|BreakItem_S _returnvalue)) (.CanCraft? (Utilities|Struct|BreakItem_S _returnvalue)) (.ResourcesNeeded (Utilities|Struct|BreakItem_S _returnvalue))))))))))

(fn ConstructionScript)